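; Example Blueprint that demonstrates writing and reading INI config values through KK-prefixed helper functions.
; The write event stores sample primitives, color, rotator, vectors and a string array in a SetValue section at FilePath, but its call is unconnected.
; BeginPlay runs the read event, printing the stored color and array, the GameUserSettings directory, config file names and the file's section names.
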(event `KK_Write`
  (bind _file_path (`self.file_path`))
  (bind _file_path_2 (`self.file_path`))
  ;[0 0.9062 1] write
  (`|ExecutionSequence`
    (:`then_0`
      (`KKConfigBlueprintFunctionLibrary.KK_SetValueToIni_Bool` _file_path "SetValue" "boolV" true)
      (`KKConfigBlueprintFunctionLibrary.KK_SetValueToIni_Float` _file_path "SetValue" "floatV" 12.412)
      (`KKConfigBlueprintFunctionLibrary.KK_SetValueToIni_Int` _file_path "SetValue" "intV" 124)
      (`KKConfigBlueprintFunctionLibrary.KK_SetValueToIni_String` _file_path "SetValue" "stringV" "this is string"))
    (:`then_1`
      (`KKConfigBlueprintFunctionLibrary.KK_SetValueToIni_Color` _file_path_2 "SetValue" "colorV" (`KismetMathLibrary.Conv_LinearColorToColor` (struct :`R` 0.875 :`G` 0.71039 :`B` 0.514286 :`A` 1.0)))
      (`KKConfigBlueprintFunctionLibrary.KK_SetValueToIni_Rotator` _file_path_2 "SetValue" "rotatorV" (struct :`Pitch` 123.0 :`Yaw` 56.0 :`Roll` 124.0))
      (`KKConfigBlueprintFunctionLibrary.KK_SetValueToIni_Vector` _file_path_2 "SetValue" "v3" (12.0 1244.0 250.0))
      (`KKConfigBlueprintFunctionLibrary.KK_SetValueToIni_Vector2` _file_path_2 "SetValue" "v2" (124.0 2140.0))
      (`KKConfigBlueprintFunctionLibrary.KK_SetValueToIni_Vector4` _file_path_2 "SetValue" "v4" (`KismetMathLibrary.MakeVector4` 44.0 35.0 35.0 2355.235107))
      (`KKConfigBlueprintFunctionLibrary.KK_SetValueToIni_Array` _file_path_2 "SetValue" "arrayV" (`|MakeArray` "A" "B" "C" "D")))))

(event `self.ReceiveBeginPlay`
  (`self.KK_Read`))

(event `KK_Read`
  (bind _file_path (`self.file_path`))
  (`|ExecutionSequence`
    (:`then_0`
      (`KismetSystemLibrary.PrintString` (`KismetStringLibrary.Conv_ColorToString` (`KismetMathLibrary.Conv_ColorToLinearColor` (`KKConfigBlueprintFunctionLibrary.KK_GetValueFromIni_Color` _file_path "SetValue" "colorV"))))
      (for _array_element (`KKConfigBlueprintFunctionLibrary.KK_GetValueFromIni_Array` _file_path "SetValue" "arrayV")
        (`KismetSystemLibrary.PrintString` _array_element)))
    (:`then_1`
      (`KismetSystemLibrary.PrintString` (`KKConfigBlueprintFunctionLibrary.KK_GetGameUserSettingsDir`))
      (`KismetSystemLibrary.PrintString` "-----------------")
      (for _array_element_2 (`KKConfigBlueprintFunctionLibrary.KK_GetConfigFileNameList`)
        (`KismetSystemLibrary.PrintString` _array_element_2)))
    (:`then_2`
      (`KismetSystemLibrary.PrintString` "-----------------")
      (for _array_element_3 (`KKConfigBlueprintFunctionLibrary.KK_GetSectionNameList` (`self.file_path`))
        (`KismetSystemLibrary.PrintString` _array_element_3)))))

(fn `UserConstructionScript`)